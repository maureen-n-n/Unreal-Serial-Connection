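; BP_LEDManager sends keyboard-triggered values over a serial port, apparently to switch an external LED.
; On BeginPlay it constructs and stores a COM_Manager object and starts reading a hard-coded COM port.
; The 0 and 1 keys call the LEDmanager function, which sends that number as an integer through the manager and prints it.
; No graph here handles incoming serial data.
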(event EventBeginPlay
  (bind _returnvalue (Game|ConstructObjectfromClass "/Script/COM_Tools.COM_Manager"))
  (bind _output_get (Variables|Default|SetNewVar _returnvalue))
  (Class|COMManager|StartReadingSerialPort _output_get "COM8" 115200 false 8 1))

(event Input|KeyboardEvents|1
  (params (Key :type Key%20Structure :default "None"))
  (:Pressed
    (CallFunction|LEDmanager 1)))

(event Input|KeyboardEvents|0
  (params (Key :type Key%20Structure :default "None"))
  (:Pressed
    (CallFunction|LEDmanager)))

(fn ConstructionScript)

(fn LEDmanager
  (params (KeyboardInput :type Integer))
  (Class|COMManager|SendSerialValueasInt (Variables|Default|GetNewVar) "COM8" 115200 KeyboardInput false 8 1)
  (Development|PrintString (Utilities|String|ToString(Integer) KeyboardInput)))