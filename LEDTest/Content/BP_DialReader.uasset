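; BP_DialReader reads two dial values from an external device over a serial port.
; On BeginPlay it creates a COM_Manager, opens COM5 with fixed settings and debug on, and binds a data-received event.
; Each received string is split on commas into Dial1 and Dial2 integers, which are printed to screen, and the port reading stops on EndPlay.
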(event Custom|OnSerialDataReceived_Event
  (params (Data :type String))
  (bind _returnvalue (Utilities|String|ParseIntoArray Data ","))
  (Variables|Default|SetDial_1 (Math|Conversions|ToInteger(Byte) (Utilities|Array|Get(acopy) _returnvalue)))
  (Variables|Default|SetDial_2 (Math|Conversions|ToInteger(Byte) (Utilities|Array|Get(acopy) _returnvalue 1)))
  (Development|PrintString (Utilities|String|Append (Utilities|String|ToString(Integer) (Variables|Default|GetDial_1)) "|" (Utilities|String|ToString(Integer) (Variables|Default|GetDial_2))) true true "(R=1.000000,G=0.000000,B=0.245794,A=1.000000)"))

(event EventBeginPlay
  (Development|PrintString "Hello")
  (bind _returnvalue (Game|ConstructObjectfromClass "/Script/COM_Tools.COM_Manager"))
  (bind _output_get (Variables|Default|SetNewVar _returnvalue))
  (Class|COMManager|StartReadingSerialPort _output_get "COM5" 115200 true 8 1)
  (EventDispatchers|AssignOnSerialDataReceived _output_get (delegate Custom|OnSerialDataReceived_Event)))

(event EventEndPlay
  (params (EndPlayReason :type EEndPlayReason%20Enum :default "Destroyed"))
  (Class|COMManager|StopReadingSerialPort (Variables|Default|GetNewVar) false))

(fn ConstructionScript)